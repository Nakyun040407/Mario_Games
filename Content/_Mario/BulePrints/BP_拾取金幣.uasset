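; A coin pickup actor that adds coins to the player when collected.
; On BeginPlay it casts and caches the first player controller as BP_玩家控制器.
; When the player character overlaps its Sphere, it passes its coin amount variable to that controller's 增加金幣 (add coins) function.
; It then plays the Mario coin sound, spawns an explosion emitter at its location and destroys itself.
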(event `self.ReceiveBeginPlay`
  ;[1 1 1] 建立玩家控制器參考
  (bind `_asbp_玩家控制器` (cast `/Game/_Mario/BulePrints/BP_玩家控制器` (`GameplayStatics.GetPlayerController` 0)))
  (set `self.BP 玩家控制器` `_asbp_玩家控制器`))

(event `self.Sphere.OnComponentBeginOverlap`
  (params (OverlappedComponent :type "PrimitiveComponent Object Reference") (OtherActor :type "Actor Object Reference") (OtherComp :type "PrimitiveComponent Object Reference") (OtherBodyIndex :type Integer) (bFromSweep :type Boolean) (SweepResult :type "HitResult Structure (by ref)"))
  ;[1 1 1] 增加金幣腳本
  (if (== OtherActor (`GameplayStatics.GetPlayerCharacter` 0))
    (`/Game/_Mario/BulePrints/BP_玩家控制器.增加金幣` (`self.BP 玩家控制器`) (`self.硬幣增加`))
    (`GameplayStatics.PlaySound2D` "/Game/_Mario/Audio/Audio/Mario_Coin.Mario_Coin" 1.0 1.0 0.0 null null)
    (`GameplayStatics.SpawnEmitterAtLocation` "/Game/StarterContent/Particles/P_Explosion.P_Explosion" (`self.K2_GetActorLocation`))
    (`self.K2_DestroyActor`)))

(fn `UserConstructionScript`)