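; Breakable brick block for a Mario-style game that awards points and disappears when hit.
; The hit event plays an interaction sound and particle effect just above the block, then spawns an actor at its transform carrying the score value.
; It adds the same points through the player controller, then destroys itself.
; BeginPlay, Tick and overlap events are disabled stubs, so all logic runs from that hit event.
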(event `/Game/_Mario/BulePrints/BPI_平台遊戲.擊中區塊`
  (`|ExecutionSequence`
    (:`then_0`
      (`/Game/_Mario/BulePrints/BP_函數庫.遊戲區互動特效` (`self.互動聲音特效`) null (`self.互動特效(Particle)`) (+ (`self.K2_GetActorLocation`) (0.0 0.0 50.0))))
    (:`then_1`
      (`|SpawnActorFromClass` "/Game/_Mario/BulePrints/BP_積分.BP_積分_C" (`self.GetTransform`) "Undefined" "MultiplyWithRoot" null (`self.積分`) null)
      (`/Game/_Mario/BulePrints/BP_玩家控制器.增加積分` (`self.玩家控制器`) (`self.積分`)))
    (:`then_2`
      (`self.K2_DestroyActor`))))

(fn `UserConstructionScript`
  (`parent.UserConstructionScript`))