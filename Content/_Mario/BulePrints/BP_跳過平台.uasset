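; BP_跳過平台 is a one-way platform that the player can jump up through or drop down from.
; Overlapping the lower box (下方碰撞框) disables collision on 平台, and leaving it restores collision.
; The upper box (上方碰撞框) flags the player as standing on top, letting the IA_玩家往下 down input disable collision.
; Both boxes respond only to player character 0.
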(event `self.下方碰撞框.OnComponentBeginOverlap`
  (params (OverlappedComponent :type "PrimitiveComponent Object Reference") (OtherActor :type "Actor Object Reference") (OtherComp :type "PrimitiveComponent Object Reference") (OtherBodyIndex :type Integer) (bFromSweep :type Boolean) (SweepResult :type "HitResult Structure (by ref)"))
  ;[1 1 1] 往上跳穿過平台
  (if (== OtherActor (`GameplayStatics.GetPlayerCharacter` 0))
    (`PrimitiveComponent.SetCollisionEnabled` (`self.平台`) "NoCollision")))

(event `self.下方碰撞框.OnComponentEndOverlap`
  (params (OverlappedComponent :type "PrimitiveComponent Object Reference") (OtherActor :type "Actor Object Reference") (OtherComp :type "PrimitiveComponent Object Reference") (OtherBodyIndex :type Integer))
  ;[1 1 1] 往上跳穿過平台
  (if (== (`GameplayStatics.GetPlayerCharacter` 0) OtherActor)
    (`PrimitiveComponent.SetCollisionEnabled` (`self.平台`) "QueryAndPhysics")))

(event `self.上方碰撞框.OnComponentBeginOverlap`
  (params (OverlappedComponent :type "PrimitiveComponent Object Reference") (OtherActor :type "Actor Object Reference") (OtherComp :type "PrimitiveComponent Object Reference") (OtherBodyIndex :type Integer) (bFromSweep :type Boolean) (SweepResult :type "HitResult Structure (by ref)"))
  ;[1 1 1] 是否在平台上
  (if (== OtherActor (`GameplayStatics.GetPlayerCharacter` 0))
    (set `self.是否在上方平台` true)))

(event `self.上方碰撞框.OnComponentEndOverlap`
  (params (OverlappedComponent :type "PrimitiveComponent Object Reference") (OtherActor :type "Actor Object Reference") (OtherComp :type "PrimitiveComponent Object Reference") (OtherBodyIndex :type Integer))
  ;[1 1 1] 是否在平台上
  (if (== (`GameplayStatics.GetPlayerCharacter` 0) OtherActor)
    (set `self.是否在上方平台` false)))

(event `EnhancedInput|/Game/ThirdPerson/Input/IA_玩家往下`
  (params (ActionValue :type Boolean) (ElapsedSeconds :type "Float (double-precision)") (TriggeredSeconds :type "Float (double-precision)") (InputAction :type "InputAction Object Reference" :default "/Game/ThirdPerson/Input/IA_玩家往下.IA_玩家往下"))
  (:`Started`
    (if (`self.是否在上方平台`)
      (`PrimitiveComponent.SetCollisionEnabled` (`self.平台`) "NoCollision"))))

(fn `UserConstructionScript`)