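; Mario-style brick block actor that gives a one-time reward when its hit event (擊中區塊) fires.
; The first hit plays interaction effects, swaps the cube material, spawns score and coin actors, and adds both values to the player controller.
; A timeline bumps the cube along its relative Z axis.
; A completion flag then limits later hits to a bump sound only.
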(event `self.擊中區塊`
  (if (`self.完成互動?`)
    (`GameplayStatics.PlaySound2D` "/Game/_Mario/Audio/Audio/Mario_BrickBump.Mario_BrickBump" 1.0 1.0 0.0 null null)
    (else
      (`|ExecutionSequence`
        (:`then_0`
          ;[1 1 1] 0.播放特效
          (`/Game/_Mario/BulePrints/BP_函數庫.遊戲區互動特效` (`self.互動聲音特效`) null (`self.互動特效(Particle)`) (+ (`self.K2_GetActorLocation`) (0.0 0.0 50.0)))
          (`PrimitiveComponent.SetMaterial` (`self.Cube`) 0 (`self.互動材質`)))
        (:`then_1`
          ;[1 1 1] 1.增加點數
          (`|SpawnActorFromClass` "/Game/_Mario/BulePrints/BP_積分.BP_積分_C" (`self.GetTransform`) "Undefined" "MultiplyWithRoot" null (`self.積分`) null)
          (`/Game/_Mario/BulePrints/BP_玩家控制器.增加積分` (`self.玩家控制器`) (`self.積分`)))
        (:`then_2`
          ;[1 1 1] 2.增加硬幣
          (`|SpawnActorFromClass` "/Game/_Mario/BulePrints/BP_磚塊_硬幣.BP_磚塊_硬幣_C" (`self.GetTransform`) "Undefined" "MultiplyWithRoot" null null)
          (`/Game/_Mario/BulePrints/BP_玩家控制器.增加金幣` (`self.玩家控制器`) (`self.要增加的硬幣`)))
        (:`then_3`
          ;[1 1 1] 3.磚塊動畫
          (bind (_direction `_移動`) (`Timeline|磚塊動畫` :!via `PlayFromStart`)
            (:`Update`
              (`SceneComponent.K2_SetRelativeLocation` (`self.Cube`) (`KismetMathLibrary.MakeVector` 0.0 0.0 `_移動`) false false))))
        (:`then_4`
          (set `self.完成互動?` true))))))

(fn `UserConstructionScript`
  (`parent.UserConstructionScript`))