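; Base brick Blueprint for a Mario-style game that reacts when the player character bumps it vertically.
; On BeginPlay it caches the player controller as BP_玩家控制器, though this graph does not use it further.
; The Cube's hit event filters for the player character and an impact normal Z of exactly 1, then sends the 擊中區塊 (block hit) message, with no response implemented here.
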(event `self.ReceiveBeginPlay`
  (bind `_asbp_玩家控制器` (cast `/Game/_Mario/BulePrints/BP_玩家控制器` (`GameplayStatics.GetPlayerController` 0)))
  (set `self.玩家控制器` `_asbp_玩家控制器`))

(event `self.Cube.OnComponentHit`
  (params (HitComponent :type "PrimitiveComponent Object Reference") (OtherActor :type "Actor Object Reference") (OtherComp :type "PrimitiveComponent Object Reference") (NormalImpulse :type "Vector Structure") (Hit :type "HitResult Structure (by ref)"))
  (if (and (== OtherActor (`GameplayStatics.GetPlayerCharacter` 0)) (== (.z (`.ImpactNormal` (`GameplayStatics.BreakHitResult` Hit))) 1.0))
    (message `/Game/_Mario/BulePrints/BPI_平台遊戲.擊中區塊` self)))

(fn `UserConstructionScript`)