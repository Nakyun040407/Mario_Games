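; BP_積分 is a short-lived score popup actor in the Mario project that displays the points added (增加的積分).
; On BeginPlay it gets the WBP_積分 widget from its Widget component, plays the 積分動畫 animation and sets the text to the points value.
; It then waits for the animation's end time and destroys itself.
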(event `self.ReceiveBeginPlay`
  (bind `_aswbp_積分` (cast `/Game/_Mario/UI/WBP_積分` (`WidgetComponent.GetWidget` (`self.Widget`))))
  (bind `_積分動畫` (`/Game/_Mario/UI/WBP_積分.積分動畫` `_aswbp_積分`))
  (`UserWidget.PlayAnimation` `_aswbp_積分` `_積分動畫` 0.0 1 "Forward" 1.0 false)
  (`TextBlock.SetText` (`/Game/_Mario/UI/WBP_積分.積分文字` `_aswbp_積分`) (`KismetTextLibrary.Conv_IntToText` (`self.增加的積分`)))
  (`KismetSystemLibrary.Delay` (`WidgetAnimation.GetEndTime` `_積分動畫`))
  (`self.K2_DestroyActor`))

(fn `UserConstructionScript`)