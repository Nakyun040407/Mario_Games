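; Coin actor for a Mario game, named as a brick coin, that plays a one-shot pop animation when spawned and then removes itself.
; On BeginPlay, a timeline drives the coin component's relative Z offset and its pitch rotation.
; When the timeline finishes, it spawns a loot pickup particle at the coin's world location and destroys the actor.
; It has no active overlap or scoring logic.
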(event `self.ReceiveBeginPlay`
  (`TimelineComponent.SetPlayRate` (`self.硬幣動畫`) 1.0)
  (bind (_direction `_移動` `_旋轉`) (`Timeline|硬幣動畫` :!via `PlayFromStart`)
    (:`Update`
      (`SceneComponent.K2_SetRelativeLocationAndRotation` (`self.硬幣`) (`KismetMathLibrary.MakeVector` 0.0 0.0 `_移動`) (`KismetMathLibrary.MakeRotator` 0.0 `_旋轉`) false false))
    (:`Finished`
      (`GameplayStatics.SpawnEmitterAtLocation` "/Game/InfinityBladeEffects/Effects/FX_Treasure/Loot/P_Loot_Pickup.P_Loot_Pickup" (`SceneComponent.K2_GetComponentLocation` (`self.硬幣`)))
      (`self.K2_DestroyActor`))))

(fn `UserConstructionScript`)