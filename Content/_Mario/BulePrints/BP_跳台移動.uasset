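; Moving jump platform that travels between a start and an end position in the level.
; On BeginPlay it plays a timeline at a configurable play rate, whose track drives a vector lerp between the two positions.
; Each update sets the platform component's relative location without sweep or teleport; Tick and overlap events are unused.
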(event `self.ReceiveBeginPlay`
  (`parent.ReceiveBeginPlay`)
  (`TimelineComponent.SetPlayRate` (`self.平台移動`) (`self.播放速率`))
  (bind (_direction `_新建轨道_0`) (`Timeline|平台移動`)
    (:`Update`
      (`SceneComponent.K2_SetRelativeLocation` (`self.平台`) (`KismetMathLibrary.VLerp` (`self.開始位置`) (`self.結束位置`) `_新建轨道_0`) false false))))

(fn `UserConstructionScript`
  (`parent.UserConstructionScript`))