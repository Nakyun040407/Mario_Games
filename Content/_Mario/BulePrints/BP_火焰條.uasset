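; Mario-style fire bar: a rotating row of fireballs, built in the Construction Script from configurable count, spacing, size and rotation rate.
; Each loop pass adds an instanced mesh along local Z, moves the Box to half the current length, and sets the RotatingMovement rate.
; The node that would resize the Box extent is unconnected, so only its position follows the length.
; The event graph has no active logic, including overlap handling.
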(fn `UserConstructionScript`
  (for _index (range (`self.火焰求數量`))
    (`|ExecutionSequence`
      (:`then_0`
        (bind _returnvalue (* _index (`self.火焰球間距`)))
        ;[1 1 1] 增加火焰球實例
        (`InstancedStaticMeshComponent.AddInstance` (`self.InstancedStaticMesh`) (`KismetMathLibrary.MakeTransform` (`KismetMathLibrary.MakeVector_NetQuantize` 0.0 0.0 (`KismetMathLibrary.Conv_IntToDouble` _returnvalue)) (struct) (`self.火焰球尺寸`)) false))
      (:`then_1`
        ;[1 1 1] 碰撞框範圍大小
        (`SceneComponent.K2_SetRelativeLocation` (`self.Box`) (`KismetMathLibrary.MakeVector` 0.0 0.0 (`KismetMathLibrary.Conv_IntToDouble` (/ _returnvalue 2))) false false))
      (:`then_2`
        ;[1 1 1] 自訂選轉速率
        (set `RotatingMovementComponent.RotationRate` (`self.旋轉速率`) (`self.RotatingMovement`))))))