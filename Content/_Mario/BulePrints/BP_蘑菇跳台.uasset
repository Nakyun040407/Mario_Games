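; Mushroom jump pad that launches the player and spawns a burst effect when they land squarely on the cap.
; A DoOnce gates each bounce, while a timeline pulses the cap's scale and re-arms the gate through a delay.
; Overlapping the bottom box disables cap collision; the logic to restore it is disconnected.
; The construction script sizes the cap and stacks stalk instances downward to match the endpoint vector's length.
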(event `self.底部碰撞框.OnComponentBeginOverlap`
  (params (OverlappedComponent :type "PrimitiveComponent Object Reference") (OtherActor :type "Actor Object Reference") (OtherComp :type "PrimitiveComponent Object Reference") (OtherBodyIndex :type Integer) (bFromSweep :type Boolean) (SweepResult :type "HitResult Structure (by ref)"))
  (if (== OtherActor (`GameplayStatics.GetPlayerCharacter` 0))
    (`PrimitiveComponent.SetCollisionEnabled` (`self.蘑菇頭`) "NoCollision")))

(event `self.底部碰撞框.OnComponentEndOverlap`
  (params (OverlappedComponent :type "PrimitiveComponent Object Reference") (OtherActor :type "Actor Object Reference") (OtherComp :type "PrimitiveComponent Object Reference") (OtherBodyIndex :type Integer)))

(event `重設蘑菇頭彈跳一次`
  (goto _label :!via `Reset`))

(event `self.蘑菇頭.OnComponentHit`
  (params (HitComponent :type "PrimitiveComponent Object Reference") (OtherActor :type "Actor Object Reference") (OtherComp :type "PrimitiveComponent Object Reference") (NormalImpulse :type "Vector Structure") (Hit :type "HitResult Structure (by ref)"))
  (bind _returnvalue (`GameplayStatics.GetPlayerCharacter` 0))
  (bind (_bblockinghit _binitialoverlap _time _distance _location _impactpoint _normal _impactnormal) (`GameplayStatics.BreakHitResult` Hit))
  (if (and (== OtherActor _returnvalue) (`KismetMathLibrary.EqualExactly_VectorVector` _impactnormal (0.0 0.0 -1.0)))
    (`/Engine/EditorBlueprintResources/StandardMacros.DoOnce` false :!label _label
      (:`Completed`
        (`Character.LaunchCharacter` _returnvalue (`self.跳躍速度`) false false)
        (`GameplayStatics.SpawnEmitterAtLocation` "/Game/InfinityBladeEffects/Effects/FX_Skill_Leap/P_Skill_Leap_Base_Launch.P_Skill_Leap_Base_Launch" _impactpoint (struct) (3.0 3.0 3.0))
        (bind (_direction `_縮放值`) (`Timeline|蘑菇頭縮放變化`)
          (:`Update`
            (`SceneComponent.SetRelativeScale3D` (`self.蘑菇頭`) (`KismetMathLibrary.MakeVector` (* (`self.蘑菇頭_X比例`) `_縮放值`) (* (`self.蘑菇頭_Y比例`) `_縮放值`) (* (`self.蘑菇頭_Z比例`) `_縮放值`)))
            (`KismetSystemLibrary.Delay` 0.2)
            (`self.重設蘑菇頭彈跳一次`)))))))

(fn `UserConstructionScript`
  (`SceneComponent.SetWorldScale3D` (`self.蘑菇頭`) (`KismetMathLibrary.MakeVector` (`self.蘑菇頭_X比例`) (`self.蘑菇頭_Y比例`) (`self.蘑菇頭_Z比例`)))
  (for _index (range (+ (`KismetMathLibrary.FTrunc` (/ (`KismetMathLibrary.VSize` (`self.蘑菇柄端點`)) 100.0)) 1))
    (`InstancedStaticMeshComponent.AddInstance` (`self.蘑菇柄`) (`KismetMathLibrary.MakeTransform` (`KismetMathLibrary.MakeVector` 0.0 0.0 (* _index -100.0))) false)))