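; Player controller for a Mario-style game that holds the player's coins, lives and score and shows the HUD.
; BeginPlay creates the WBP_HUD widget and adds it to the viewport.
; The add-coins event (增加金幣) rolls the clamped count over at 100, granting a life and playing the 1-up sound.
; The add-score event (增加積分) simply accumulates points.
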(event `self.ReceiveBeginPlay`
  (bind _returnvalue (`|CreateWidget` "/Game/_Mario/BulePrints/WBP_HUD.WBP_HUD_C"))
  (`UserWidget.AddToViewport` _returnvalue 0))

(event `增加金幣`
  (params (`硬幣增加` :type Integer))
  (bind _returnvalue (+ `硬幣增加` (`self.金幣`)))
  ;[1 1 1] 增加金幣腳本
  (if (>= _returnvalue 100)
    (set `self.金幣` (`KismetMathLibrary.Clamp` (- _returnvalue 100) 0 100))
    (`/Engine/EditorBlueprintResources/StandardMacros.IncrementInt` (`self.生命`)
      (:`  `
        (`GameplayStatics.PlaySound2D` "/Game/_Mario/Audio/Audio/Mario_1up.Mario_1up" 1.0 1.0 0.0 null null)))
    (else
      (set `self.金幣` (`KismetMathLibrary.Clamp` _returnvalue 0 100)))))

(event `增加積分`
  (params (`增加的積分` :type Integer))
  ;[1 1 1] 增加積分
  (set `self.積分` (+ `增加的積分` (`self.積分`))))

(fn `UserConstructionScript`)